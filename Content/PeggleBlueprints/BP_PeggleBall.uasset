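; Peggle ball actor that launches forward on spawn, with material and explosion color set by ball type; duds ignore WorldDynamic so they skip pegs.
; When a non-dud ball stalls, a reversible heat timeline ramps its glow and warning sound, exploding it when full.
; That ends the shot, resetting player state and destroying other balls.
; Hits play speed-scaled bump sounds; the kill-volume overlap and per-type sound logic are disconnected.
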(event OnComponentBeginOverlap(StaticMesh)
  (params (OverlappedComponent :type Primitive%20Component%20Object%20Reference) (OtherActor :type Actor%20Object%20Reference) (OtherComp :type Primitive%20Component%20Object%20Reference) (OtherBodyIndex :type Integer) (bFromSweep :type Boolean) (SweepResult :type Hit%20Result%20Structure%20%28by%20ref%29))
  ;[1 1 1] Kill the ball when it goes through the kill volume off screen. (Careful as it will kill it no matter what kind of volume it is. Maybe give it a tag?)
)

(event OnComponentHit(StaticMesh)
  (params (HitComponent :type Primitive%20Component%20Object%20Reference) (OtherActor :type Actor%20Object%20Reference) (OtherComp :type Primitive%20Component%20Object%20Reference) (NormalImpulse :type Vector :default "0, 0, 0") (Hit :type Hit%20Result%20Structure%20%28by%20ref%29))
  ;[1 1 1] Play bump sound effect when it hits stuff. (Some logic to keep it from rapidly spamming sfx while rolling on an object or hiting it really fast.) Also some to modulate volume based on hit speed.
  (if (not (== HitComponent (Variables|Default|GetHit%20Component)))
    (Variables|Default|SetHit%20Component HitComponent)
    (bind _returnvalue (Physics|GetPhysicsLinearVelocity (Variables|Default|GetStaticMesh) "None"))
    ;[1 1 1] Currently a different sound based on ball type, but will probably narrow down to one.
    (Audio|PlaySound2D "/Game/PeggleAssets/Sounds/UISounds/switch10.switch10" (* (Math|Vector|VectorLength _returnvalue) 0.001) 1.0 0.075 0 0)
    (Utilities|FlowControl|Delay 0.2)
    (Variables|Default|SetHit%20Component (Variables|Default|GetBlankHitComponent))))

(event EventBeginPlay
  (bind _staticmesh (Variables|Default|GetStaticMesh))
  ;[1 1 1] If it's a dud ball, don't collide with pegs.
  (if (Variables|Default|GetIsDud?)
    (Collision|SetCollisionResponsetoChannel (Variables|Default|GetStaticMesh) "ECC_WorldDynamic" "ECR_Ignore"))
  ;[1 1 1] Makes the ball shoot out with force
  (Physics|AddImpulse _staticmesh (* (Math|Vector|GetForwardVector _staticmesh) 1e+03) "None" true)
  ;[1 1 1] Create dynamic material for heat mechanic and save color
  (bind _returnvalue (Rendering|Material|CreateDynamicMaterialInstance (Variables|Default|GetStaticMesh) 0 0 "None" :!class /Script/Engine.PrimitiveComponent))
  (bind _output_get (Variables|Default|SetDynamicMaterial _returnvalue))
  (bind _returnvalue_2 (Rendering|Material|GetVectorParameterValue _output_get "Color" :!class /Script/Engine.MaterialInstanceDynamic))
  (Variables|Default|SetBallMATColor _returnvalue_2)
  ;[1 1 1] Spawn the heat warning sound but keep it silent and store it as a variable
  (bind _returnvalue_3 (Audio|SpawnSound2D "/Game/Interface_and_Item_SFX_10/Items_Collectibles/cue/Coins__15__Cue.Coins__15__Cue" 0.0 1.0 0.0 0))
  (Variables|Default|SetExplodeDamgerSound _returnvalue_3))

(event EventTick
  (params (DeltaSeconds :type Float%20%28single-precision%29))
  (bind _explodedamgersound (Variables|Default|GetExplodeDamgerSound))
  (bind _dynamicmaterial (Variables|Default|GetDynamicMaterial))
  (bind _minspeed (Variables|Default|GetMinSpeed))
  (bind _returnvalue (* _minspeed -1.0))
  ;[1 1 1] Check if ball has stopped moving. If not, set switch off. If so, set the switch on and delay then check if the switch is still on. If so, kill the ball. (This is janky and sometimes kills moving balls)
  (if (Utilities|Enum|NotEqual(Enum) (Variables|Default|GetBallType) "NewEnumerator11")
    (bind _returnvalue_2 (Physics|GetPhysicsLinearVelocity (Variables|Default|GetStaticMesh) "None"))
    (if (Math|Boolean|ANDBoolean (Math|Float|InRange(Float) (.X (Math|Vector|BreakVector _returnvalue_2)) _returnvalue _minspeed) (Math|Float|InRange(Float) (.Y (Math|Vector|BreakVector _returnvalue_2)) _returnvalue _minspeed) (Math|Float|InRange(Float) (.Z (Math|Vector|BreakVector _returnvalue_2)) _returnvalue _minspeed))
      (Variables|Default|SetStopped? true)
      (bind _heat (Timeline|BallHeat Play)
        (:Update
          ;[1 1 1] Set the pitch and volume of the heat warning sound. If it's low, set to zero.
          (if (<= _heat 0.2)
            (Audio|Components|Audio|SetPitchMultiplier _explodedamgersound 0.0)
            (Audio|Components|Audio|SetVolumeMultiplier _explodedamgersound 0.0 :!class /Script/Engine.AudioComponent)
            (else
              (Audio|Components|Audio|SetPitchMultiplier _explodedamgersound (+ _heat 0.2))
              (Audio|Components|Audio|SetVolumeMultiplier _explodedamgersound (+ _heat 0.2) :!class /Script/Engine.AudioComponent)))
          (Rendering|Material|SetVectorParameterValue _dynamicmaterial "Color" (Math|Color|Lerp(LinearColor) (Variables|Default|GetBallMATColor) (Variables|Default|GetBallHeatMATColor) _heat) :!class /Script/Engine.MaterialInstanceDynamic)
          (Rendering|Material|SetScalarParameterValue _dynamicmaterial "Emissive" _heat :!class /Script/Engine.MaterialInstanceDynamic)
          (if (Math|Boolean|ANDBoolean (Math|Float|InRange(Float) (.X (Math|Vector|BreakVector _returnvalue_2)) _returnvalue _minspeed) (Math|Float|InRange(Float) (.Y (Math|Vector|BreakVector _returnvalue_2)) _returnvalue _minspeed) (Math|Float|InRange(Float) (.Z (Math|Vector|BreakVector _returnvalue_2)) _returnvalue _minspeed))
            (Variables|Default|SetStopped? true)
            (else
              (Variables|Default|SetStopped? false)
              (Timeline|BallHeat Reverse))))
        (:Finished
          (if (>= _heat 0.9)
            (CallFunction|Explode)
            (CallFunction|EndShot)
            (CallFunction|DestroyBall))))
      (else
        (Variables|Default|SetStopped? false)))))

(fn ConstructionScript
  ;[1 1 1] Set the ball material to the proper color based on ball type that was set when spawned.
  (Rendering|Material|SetMaterial (Variables|Default|GetStaticMesh) 0 (Utilities|Select :Index (Variables|Default|GetBallType) :NewEnumerator1 "/Game/PeggleAssets/PegMaterials/M_PegPassion.M_PegPassion" :NewEnumerator2 "/Game/PeggleAssets/PegMaterials/M_PegFlirtation.M_PegFlirtation" :NewEnumerator3 "/Game/PeggleAssets/PegMaterials/M_PegRomance.M_PegRomance" :NewEnumerator4 "/Game/PeggleAssets/PegMaterials/M_PegSexuality.M_PegSexuality" :NewEnumerator5 "/Game/PeggleAssets/PegMaterials/M_PegTalent.M_PegTalent" :NewEnumerator11 "/Game/PeggleAssets/PegMaterials/M_PegBlocker.M_PegBlocker")))

(fn EndShot
  (bind _returnvalue (Game|Player|GetPlayerPawn 0))
  (bind _asbp_peggle_player (Utilities|Casting|CastToBP_PegglePlayer _returnvalue))
  ;[1 1 1] If it's not a dud ball
  (if (Utilities|Enum|NotEqual(Enum) (Variables|Default|GetBallType) "NewEnumerator11")
    ;[1 1 1] Get the player, set the next ball type, number of dud balls, and preview ball material. Then destroy all other balls onscreen. (Which SHOULD only be dud balls hopefully.)
    (Variables|/Game/PeggleBlueprints/BP_PegglePlayer.BP_PegglePlayer_C|SetBallInPlay? _asbp_peggle_player false)
    (Variables|/Game/PeggleBlueprints/BP_PegglePlayer.BP_PegglePlayer_C|SetNextBallType _asbp_peggle_player (Variables|/Game/PeggleBlueprints/BP_PegglePlayer.BP_PegglePlayer_C|GetLastBallType _asbp_peggle_player))
    (Variables|/Game/PeggleBlueprints/BP_PegglePlayer.BP_PegglePlayer_C|SetNumberOfDuds _asbp_peggle_player 0)
    (Variables|/Game/PeggleBlueprints/BP_PegglePlayer.BP_PegglePlayer_C|SetComboHitNumber _asbp_peggle_player 0)
    (Default|SetPreviewBallColor _asbp_peggle_player)
    (bind _outactors (Actor|GetAllActorsOfClass "BP_PeggleBall_C"))
    (for _array_element _outactors
      (if (!= _array_element self)
        (CallFunction|Explode _array_element)
        (CallFunction|DestroyBall _array_element)))))

(fn DestroyBall
  (Components|DestroyComponent (Variables|Default|GetExplodeDamgerSound))
  (Actor|DestroyActor))

(fn Explode
  ;[1 1 1] Spawn explosion actor with material matching the ball type and play some sounds
  (Game|SpawnActorfromClass "/Game/PeggleBlueprints/BP_ExplosionParticle.BP_ExplosionParticle_C" (Math|Transform|MakeTransform (Transformation|GetWorldLocation (Variables|Default|GetStaticMesh)) "0, 0, 0" "1,1,1") "Undefined" 0 (Utilities|Select :Index (Variables|Default|GetBallType) :NewEnumerator1 "/Game/PeggleAssets/ParticleMaterials/M_ParticleShardPink.M_ParticleShardPink" :NewEnumerator2 "/Game/PeggleAssets/ParticleMaterials/M_ParticleShardGreen.M_ParticleShardGreen" :NewEnumerator3 "/Game/PeggleAssets/ParticleMaterials/M_ParticleShardYellow.M_ParticleShardYellow" :NewEnumerator4 "/Game/PeggleAssets/ParticleMaterials/M_ParticleShardRed.M_ParticleShardRed" :NewEnumerator5 "/Game/PeggleAssets/ParticleMaterials/M_ParticleShardBlue.M_ParticleShardBlue" :NewEnumerator11 "/Game/PeggleAssets/ParticleMaterials/M_ParticleShardGrey.M_ParticleShardGrey") "(B=0,G=0,R=0,A=0)" "NewEnumerator0" 0)
  (Audio|PlaySound2D "/Game/Retro_8Bit_Sounds/Explosion/Cues/retro_explosion_deep_01_Cue.retro_explosion_deep_01_Cue" 1.0 1.3 0.0 0 0))