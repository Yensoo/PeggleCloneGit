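; Player for a Peggle-style game that aims and fires limited Flirtation, Romance and Sexuality balls.
; Tick points the launch arrow at the cursor with clamped angles and draws a predicted debug path.
; Input or widget clicks fire the selected type, then switch to two dud shots while that ball is in play.
; Broken bricks raise a stepped passion multiplier and add counter peg meshes colored by the last ball type.
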(event EventTick
  (params (DeltaSeconds :type Float%20%28single-precision%29))
  (bind _returnvalue (Game|GetPlayerController 0))
  (bind _arrow (Variables|Default|GetArrow))
  (bind _arrow_2 (Variables|Default|GetArrow))
  (bind _hitresult (Game|Player|GetHitResultUnderCursorbyChannel _returnvalue "TraceTypeQuery1" false))
  (bind _returnvalue_2 (Transformation|GetWorldLocation _arrow))
  (bind _impactpoint (Collision|BreakHitResult _hitresult))
  (bind _returnvalue_3 (Math|Rotator|FindLookatRotation _returnvalue_2 _impactpoint))
  ;[1 1 1] Face arrow at mouse then do some fancy clamping to keep from aiming up for forward and backward too much. (Still not perfect, as walls and pegs aim slightly forward. Need to remove visibility channel hits for those maybe.)
  (Transformation|SetWorldRotation (Variables|Default|GetArrow) (Math|Rotator|MakeRotator (.roll _returnvalue_3) (Math|Float|ClampAngle (.pitch _returnvalue_3) -2.1e+02 3e+01) (Math|Float|ClampAngle (.yaw _returnvalue_3) 0.0 1.8e+02)) false false)
  ;[1 1 1] Show path of ball
  (Class|GameplayStatics|BlueprintPredictProjectilePathbyTraceChannel (Transformation|GetWorldLocation _arrow_2) (* (Math|Vector|GetForwardVector _arrow_2) 1e+03) true 22.0 "ECC_Pawn" false 0 "ForOneFrame"))

(event EventBrickBroken
  (bind _passioncounterstart (Variables|Default|GetPassionCounterStart))
  (bind _relativelocation (Variables|/Script/Engine.SceneComponent|GetRelativeLocation _passioncounterstart))
  (bind (_x _y _z) (Math|Vector|BreakVector _relativelocation))
  ;[1 1 1] Add pegs to the passion tracker
  (Variables|Default|SetPegsDestroyed (+ (Variables|Default|GetPegsDestroyed) 1))
  (CallFunction|UpdatePassion)
  (bind _returnvalue (AddComponent|AddStaticMeshComponent false (Math|Transform|MakeTransform (Math|Vector|MakeVector (+ (* (Variables|Default|GetPegsDestroyed) 2e+01) _x) _y _z) "0.000000, 0,90.000000" "0.500000,0.500000,0.500000")))
  (Components|StaticMesh|SetStaticMesh _returnvalue "/Game/PeggleAssets/Pegs_RectanglePeg.Pegs_RectanglePeg")
  (Rendering|Material|SetMaterial _returnvalue 0 (Utilities|Select :Index (Variables|Default|GetLastBallType) :NewEnumerator2 "/Game/PeggleAssets/PegMaterials/M_PegFlirtation.M_PegFlirtation" :NewEnumerator3 "/Game/PeggleAssets/PegMaterials/M_PegRomance.M_PegRomance" :NewEnumerator4 "/Game/PeggleAssets/PegMaterials/M_PegSexuality.M_PegSexuality" :NewEnumerator11 "/Game/PeggleAssets/PegMaterials/M_PegBlocker.M_PegBlocker")))

(event EventWidgetActionButton
  (bind _arrow (Variables|Default|GetArrow))
  (bind _returnvalue (Transformation|GetWorldTransform _arrow))
  ;[1 1 1] Spawn ball at arrow facing the proper direction.
  ;;[1 1 1] Called by widget when mouse is captured and clicks can't get through
  (if (Variables|Default|GetBallInPlay?)
    ;[1 1 1] Logic if there's already a ball in play. This checks if you have dud balls to shoot and spawns them. If you've run out, it changes the preview ball back to what you last used.
    (if (> (Variables|Default|GetNumberOfDuds) 0)
      (Variables|Default|SetNumberOfDuds (- (Variables|Default|GetNumberOfDuds) 1))
      (Audio|PlaySound2D "/Game/Interface_and_Item_SFX_10/Interface/Clicks/cue/Click_Back__7__Cue.Click_Back__7__Cue" 1.0 1.0 0.0 0 0)
      (Game|SpawnActorfromClass "/Game/PeggleBlueprints/BP_PeggleBall.BP_PeggleBall_C" _returnvalue "Undefined" 0 (Variables|Default|GetNextBallType) (Utilities|Enum|Equal(Enum) (Variables|Default|GetNextBallType) "NewEnumerator11") 0)
      (if (not (> (Variables|Default|GetNumberOfDuds) 0))
        (Variables|Default|SetNextBallType (Variables|Default|GetLastBallType))
        (CallFunction|SetPreviewBallColor)))
    (else
      ;;[1 1 1] Check to make sure you have enough balls to shoot then minus one off the shot ball.
      (if (Utilities|Enum|Equal(Enum) (Variables|Default|GetNextBallType) "NewEnumerator11")
        (CallFunction|UpdateDisplayNumbers :!label _label)
        (Audio|PlaySound2D "/Game/Interface_and_Item_SFX_10/Interface/Clicks/cue/Click_Back__7__Cue.Click_Back__7__Cue" 1.0 1.0 0.0 0 0)
        (Game|SpawnActorfromClass "/Game/PeggleBlueprints/BP_PeggleBall.BP_PeggleBall_C" _returnvalue "Undefined" 0 (Variables|Default|GetNextBallType) (Utilities|Enum|Equal(Enum) (Variables|Default|GetNextBallType) "NewEnumerator11") 0)
        ;;[1 1 1] Sets BallInPlay to true after shooting if the ball isn't a dud and sets the last ball. Then sets things up to start using dud balls.
        (if (Utilities|Enum|NotEqual(Enum) (Variables|Default|GetNextBallType) "NewEnumerator11")
          (Variables|Default|SetBallInPlay? true)
          (Variables|Default|SetLastBallType (Variables|Default|GetNextBallType)))
        (Variables|Default|SetNextBallType "NewEnumerator11")
        (Variables|Default|SetNumberOfDuds 2)
        (CallFunction|SetPreviewBallColor)
        (elif (> (Utilities|Select :Index (Variables|Default|GetNextBallType) :NewEnumerator2 (Variables|Default|GetNumberOfFlirtation) :NewEnumerator3 (Variables|Default|GetNumberOfRomance) :NewEnumerator4 (Variables|Default|GetNumberOfSexuality) :NewEnumerator11 0) 0)
          (switch Utilities|FlowControl|Switch|SwitchonETypesOfBallsEnum (Variables|Default|GetNextBallType)
            (:NewEnumerator2
              (Variables|Default|SetNumberOfFlirtation (- (Utilities|Select :Index (Variables|Default|GetNextBallType) :NewEnumerator2 (Variables|Default|GetNumberOfFlirtation) :NewEnumerator3 (Variables|Default|GetNumberOfRomance) :NewEnumerator4 (Variables|Default|GetNumberOfSexuality) :NewEnumerator11 0) 1))
              (goto _label))
            (:NewEnumerator3
              (Variables|Default|SetNumberOfRomance (- (Utilities|Select :Index (Variables|Default|GetNextBallType) :NewEnumerator2 (Variables|Default|GetNumberOfFlirtation) :NewEnumerator3 (Variables|Default|GetNumberOfRomance) :NewEnumerator4 (Variables|Default|GetNumberOfSexuality) :NewEnumerator11 0) 1))
              (goto _label))
            (:NewEnumerator4
              (Variables|Default|SetNumberOfSexuality (- (Utilities|Select :Index (Variables|Default|GetNextBallType) :NewEnumerator2 (Variables|Default|GetNumberOfFlirtation) :NewEnumerator3 (Variables|Default|GetNumberOfRomance) :NewEnumerator4 (Variables|Default|GetNumberOfSexuality) :NewEnumerator11 0) 1))
              (goto _label)))
          (else
            (Audio|PlaySound2D "/Game/Interface_and_Item_SFX_10/Interface/Bonus/cue/Buzz_Error__2__Cue.Buzz_Error__2__Cue" 1.0 1.0 0.0 0 0)))))))

(event Input|ActionEvents|InputActionActionButton
  (params (Key :type Key%20Structure :default "None"))
  (bind _arrow (Variables|Default|GetArrow))
  (bind _returnvalue (Transformation|GetWorldTransform _arrow))
  ;[1 1 1] Spawn ball at arrow facing the proper direction.
  (:Pressed
    (if (Variables|Default|GetBallInPlay?)
      ;[1 1 1] Logic if there's already a ball in play. This checks if you have dud balls to shoot and spawns them. If you've run out, it changes the preview ball back to what you last used.
      (if (> (Variables|Default|GetNumberOfDuds) 0)
        (Variables|Default|SetNumberOfDuds (- (Variables|Default|GetNumberOfDuds) 1))
        (Audio|PlaySound2D "/Game/Interface_and_Item_SFX_10/Interface/Clicks/cue/Click_Back__7__Cue.Click_Back__7__Cue" 1.0 1.0 0.0 0 0)
        (Game|SpawnActorfromClass "/Game/PeggleBlueprints/BP_PeggleBall.BP_PeggleBall_C" _returnvalue "Undefined" 0 (Variables|Default|GetNextBallType) (Utilities|Enum|Equal(Enum) (Variables|Default|GetNextBallType) "NewEnumerator11") 0)
        (if (not (> (Variables|Default|GetNumberOfDuds) 0))
          (Variables|Default|SetNextBallType (Variables|Default|GetLastBallType))
          (CallFunction|SetPreviewBallColor)))
      (else
        ;;[1 1 1] Check to make sure you have enough balls to shoot then minus one off the shot ball.
        (if (Utilities|Enum|Equal(Enum) (Variables|Default|GetNextBallType) "NewEnumerator11")
          (CallFunction|UpdateDisplayNumbers :!label _label)
          (Audio|PlaySound2D "/Game/Interface_and_Item_SFX_10/Interface/Clicks/cue/Click_Back__7__Cue.Click_Back__7__Cue" 1.0 1.0 0.0 0 0)
          (Game|SpawnActorfromClass "/Game/PeggleBlueprints/BP_PeggleBall.BP_PeggleBall_C" _returnvalue "Undefined" 0 (Variables|Default|GetNextBallType) (Utilities|Enum|Equal(Enum) (Variables|Default|GetNextBallType) "NewEnumerator11") 0)
          ;;[1 1 1] Sets BallInPlay to true after shooting if the ball isn't a dud and sets the last ball. Then sets things up to start using dud balls.
          (if (Utilities|Enum|NotEqual(Enum) (Variables|Default|GetNextBallType) "NewEnumerator11")
            (Variables|Default|SetBallInPlay? true)
            (Variables|Default|SetLastBallType (Variables|Default|GetNextBallType)))
          (Variables|Default|SetNextBallType "NewEnumerator11")
          (Variables|Default|SetNumberOfDuds 2)
          (CallFunction|SetPreviewBallColor)
          (elif (> (Utilities|Select :Index (Variables|Default|GetNextBallType) :NewEnumerator2 (Variables|Default|GetNumberOfFlirtation) :NewEnumerator3 (Variables|Default|GetNumberOfRomance) :NewEnumerator4 (Variables|Default|GetNumberOfSexuality) :NewEnumerator11 0) 0)
            (switch Utilities|FlowControl|Switch|SwitchonETypesOfBallsEnum (Variables|Default|GetNextBallType)
              (:NewEnumerator2
                (Variables|Default|SetNumberOfFlirtation (- (Utilities|Select :Index (Variables|Default|GetNextBallType) :NewEnumerator2 (Variables|Default|GetNumberOfFlirtation) :NewEnumerator3 (Variables|Default|GetNumberOfRomance) :NewEnumerator4 (Variables|Default|GetNumberOfSexuality) :NewEnumerator11 0) 1))
                (goto _label))
              (:NewEnumerator3
                (Variables|Default|SetNumberOfRomance (- (Utilities|Select :Index (Variables|Default|GetNextBallType) :NewEnumerator2 (Variables|Default|GetNumberOfFlirtation) :NewEnumerator3 (Variables|Default|GetNumberOfRomance) :NewEnumerator4 (Variables|Default|GetNumberOfSexuality) :NewEnumerator11 0) 1))
                (goto _label))
              (:NewEnumerator4
                (Variables|Default|SetNumberOfSexuality (- (Utilities|Select :Index (Variables|Default|GetNextBallType) :NewEnumerator2 (Variables|Default|GetNumberOfFlirtation) :NewEnumerator3 (Variables|Default|GetNumberOfRomance) :NewEnumerator4 (Variables|Default|GetNumberOfSexuality) :NewEnumerator11 0) 1))
                (goto _label)))
            (else
              (Audio|PlaySound2D "/Game/Interface_and_Item_SFX_10/Interface/Bonus/cue/Buzz_Error__2__Cue.Buzz_Error__2__Cue" 1.0 1.0 0.0 0 0))))))))

(event Input|ActionEvents|InputActionNextButton
  (params (Key :type Key%20Structure :default "None"))
  ;[1 1 1] Switch current ball color with Next and Previous input actions. Set last ball to the same as Next ball as long it's not dud. Update preview ball material.
  (:Pressed
    (Variables|Default|SetNextBallType (Utilities|Select :Index (Variables|Default|GetNextBallType) :NewEnumerator2 "NewEnumerator4" :NewEnumerator3 "NewEnumerator2" :NewEnumerator4 "NewEnumerator3" :NewEnumerator11 "NewEnumerator11"))
    (if (Utilities|Enum|NotEqual(Enum) (Variables|Default|GetNextBallType) "NewEnumerator11")
      (Variables|Default|SetLastBallType (Variables|Default|GetNextBallType)))
    (CallFunction|SetPreviewBallColor)))

(event Input|ActionEvents|InputActionPreviousButton
  (params (Key :type Key%20Structure :default "None"))
  ;[1 1 1] Switch current ball color with Next and Previous input actions. Set last ball to the same as Next ball as long it's not dud. Update preview ball material.
  (:Pressed
    (Variables|Default|SetNextBallType (Utilities|Select :Index (Variables|Default|GetNextBallType) :NewEnumerator2 "NewEnumerator3" :NewEnumerator3 "NewEnumerator4" :NewEnumerator4 "NewEnumerator2" :NewEnumerator11 "NewEnumerator11"))
    (if (Utilities|Enum|NotEqual(Enum) (Variables|Default|GetNextBallType) "NewEnumerator11")
      (Variables|Default|SetLastBallType (Variables|Default|GetNextBallType)))
    (CallFunction|SetPreviewBallColor)))

(event Input|AxisEvents|InputAxisMoveHorizontal
  (params (AxisValue :type Float%20%28single-precision%29))
  (bind _arrow (Variables|Default|GetArrow))
  (bind _relativerotation (Variables|/Script/Engine.SceneComponent|GetRelativeRotation _arrow))
  ;[1 1 1] Rotate arrow and clamp rotation. Does nothing while mouse aiming is active.
  (Transformation|AddLocalRotation (Variables|Default|GetArrow) (Math|Rotator|MakeRotator 0.0 0.0 (* AxisValue -1.0)) false false)
  (Transformation|SetRelativeRotation (Variables|Default|GetArrow) (Math|Rotator|MakeRotator (.roll _relativerotation) (.pitch _relativerotation) (Math|Float|ClampAngle (.yaw _relativerotation) -3e+01 2.1e+02)) false false))

(fn ConstructionScript
  ;[1 1 1] Start with passion ball
  (CallFunction|SetPreviewBallColor)
  (CallFunction|UpdateDisplayNumbers))

(fn NewBallType
  ;[1 1 1] Randomize ball. LEGACY? (Should be completely replaces by choosing balls.)
  (bind _output_get (Variables|Default|SetNextBallType (Utilities|Enum|ByteToEnumETypesOfBallsEnum (Math|Conversions|ToByte(Integer) (Math|Random|RandomInteger 4)))))
  (Rendering|Material|SetMaterial (Variables|Default|GetPreviewBall) 0 (Utilities|Select :Index _output_get :NewEnumerator2 "/Game/PeggleAssets/PegMaterials/M_PegFlirtation.M_PegFlirtation" :NewEnumerator3 "/Game/PeggleAssets/PegMaterials/M_PegRomance.M_PegRomance" :NewEnumerator4 "/Game/PeggleAssets/PegMaterials/M_PegSexuality.M_PegSexuality" :NewEnumerator11 "/Game/PeggleAssets/PegMaterials/M_PegBlocker.M_PegBlocker")))

(fn SetPreviewBallColor
  ;[1 1 1] Sets the material for the preview ball based on what the next shot will be.
  (Rendering|Material|SetMaterial (Variables|Default|GetPreviewBall) 0 (Utilities|Select :Index (Variables|Default|GetNextBallType) :NewEnumerator2 "/Game/PeggleAssets/PegMaterials/M_PegFlirtation.M_PegFlirtation" :NewEnumerator3 "/Game/PeggleAssets/PegMaterials/M_PegRomance.M_PegRomance" :NewEnumerator4 "/Game/PeggleAssets/PegMaterials/M_PegSexuality.M_PegSexuality" :NewEnumerator11 "/Game/PeggleAssets/PegMaterials/M_PegBlocker.M_PegBlocker")))

(fn UpdateDisplayNumbers
  (Rendering|Components|TextRender|SetText (Variables|Default|GetFlirtationNumber) (Utilities|Text|ToText(Integer) (Variables|Default|GetNumberOfFlirtation)))
  (Rendering|Components|TextRender|SetText (Variables|Default|GetRomanceNumber) (Utilities|Text|ToText(Integer) (Variables|Default|GetNumberOfRomance)))
  (Rendering|Components|TextRender|SetText (Variables|Default|GetSexualityNumber) (Utilities|Text|ToText(Integer) (Variables|Default|GetNumberOfSexuality))))

(fn UpdatePassion
  (bind _pegsdestroyed (Variables|Default|GetPegsDestroyed))
  ;[1 1 1] Cycle through branches to find out what range the number of broken pegs is at, then assign the proper value to the multiplier.
  (if (< _pegsdestroyed 15)
    (Variables|Default|SetCurrentMultiplier 1.0)
    (elif (< _pegsdestroyed 25)
      ;[1 1 1] Debug
      (if (!= (Variables|Default|GetCurrentMultiplier) 2.0)
        (Development|PrintString "TIMES TWO!!!"))
      (Variables|Default|SetCurrentMultiplier 2.0)
      (elif (< _pegsdestroyed 30)
        (if (!= (Variables|Default|GetCurrentMultiplier) 3.0)
          (Development|PrintString "TIMES THREE!!!"))
        (Variables|Default|SetCurrentMultiplier 3.0)
        (elif (< _pegsdestroyed 33)
          (if (!= (Variables|Default|GetCurrentMultiplier) 5.0)
            (Development|PrintString "TIMES FIVE!!!"))
          (Variables|Default|SetCurrentMultiplier 5.0)
          (elif (>= _pegsdestroyed 33)
            (if (!= (Variables|Default|GetCurrentMultiplier) 1e+01)
              (Development|PrintString "TIMES TEN!!!"))
            (Variables|Default|SetCurrentMultiplier 1e+01)))))))