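; BP_PeggleBucket is the moving catch bucket in a Peggle-style game that refunds any ball it catches.
; A timeline slides the bucket horizontally across MoveDistance, with a FlipFlop on finish alternating reverse and forward playback for endless back-and-forth motion.
; Box overlap with a BP_PeggleBall increments the player's count for that ball type (Flirtation, Romance, Sexuality or Dud), ends the shot, destroys the ball and refreshes the displayed numbers.
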(event OnComponentBeginOverlap(Box)
  (params (OverlappedComponent :type Primitive%20Component%20Object%20Reference) (OtherActor :type Actor%20Object%20Reference) (OtherComp :type Primitive%20Component%20Object%20Reference) (OtherBodyIndex :type Integer) (bFromSweep :type Boolean) (SweepResult :type Hit%20Result%20Structure%20%28by%20ref%29))
  (bind _returnvalue (Game|Player|GetPlayerPawn 0))
  (bind _asbp_peggle_player (Utilities|Casting|CastToBP_PegglePlayer _returnvalue))
  ;[1 1 1] Give free ball if ball is caught
  (bind _asbp_peggle_ball (Utilities|Casting|CastToBP_PeggleBall OtherActor))
  (switch Utilities|FlowControl|Switch|SwitchonETypesOfBallsEnum (Variables|/Game/PeggleBlueprints/BP_PeggleBall.BP_PeggleBall_C|GetBallType _asbp_peggle_ball)
    (:NewEnumerator2
      (Variables|/Game/PeggleBlueprints/BP_PegglePlayer.BP_PegglePlayer_C|SetNumberOfFlirtation _asbp_peggle_player (+ (Variables|/Game/PeggleBlueprints/BP_PegglePlayer.BP_PegglePlayer_C|GetNumberOfFlirtation _asbp_peggle_player) 1)))
    (:NewEnumerator3
      (Variables|/Game/PeggleBlueprints/BP_PegglePlayer.BP_PegglePlayer_C|SetNumberOfRomance _asbp_peggle_player (+ (Variables|/Game/PeggleBlueprints/BP_PegglePlayer.BP_PegglePlayer_C|GetNumberOfRomance _asbp_peggle_player) 1)))
    (:NewEnumerator4
      (Variables|/Game/PeggleBlueprints/BP_PegglePlayer.BP_PegglePlayer_C|SetNumberOfSexuality _asbp_peggle_player (+ (Variables|/Game/PeggleBlueprints/BP_PegglePlayer.BP_PegglePlayer_C|GetNumberOfSexuality _asbp_peggle_player) 1)))
    (:NewEnumerator11
      (Variables|/Game/PeggleBlueprints/BP_PegglePlayer.BP_PegglePlayer_C|SetNumberOfDuds _asbp_peggle_player (+ (Variables|/Game/PeggleBlueprints/BP_PegglePlayer.BP_PegglePlayer_C|GetNumberOfDuds _asbp_peggle_player) 1))))
  (Default|EndShot _asbp_peggle_ball)
  (Default|DestroyBall _asbp_peggle_ball)
  (Default|UpdateDisplayNumbers _asbp_peggle_player))

(event EventBeginPlay
  ;[1 1 1] Move bucket back and forth
  (bind _horizontalpercent (Timeline|MoveBucket Play)
    (:Update
      (Transformation|SetRelativeLocation (Variables|Default|GetBucket) (Math|Vector|MakeVector (* _horizontalpercent (Variables|Default|GetMoveDistance)) 0.0 0.0) false false))
    (:Finished
      (Utilities|FlowControl|FlipFlop
        (:A
          (Variables|Default|SetMovingBack? true))
        (:B
          (Variables|Default|SetMovingBack? false)))
      (if (Variables|Default|GetMovingBack?)
        (Timeline|MoveBucket Reverse)
        (else
          (Timeline|MoveBucket Play))))))

(event Input|ActionEvents|InputActionRightClickButton
  (params (Key :type Key%20Structure :default "None")))

(fn ConstructionScript)