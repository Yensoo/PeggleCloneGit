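; Breakable Peggle peg whose type sets its material and scoring, with mesh and material applied in the construction script.
; Non-Dud ball hits pop Special pegs with effects only, ignore Blockers, and otherwise call HitByBall, which requires a color match unless Type02 is set.
; HitByBall builds score from combo, Type02 match bonus, current girl's likes/dislikes, player stat and multiplier, then updates GameInstance, notifies UI and player, and spawns effects.
; BeginPlay's color randomization is disconnected.
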(event OnComponentHit(Peg)
  (params (HitComponent :type Primitive%20Component%20Object%20Reference) (OtherActor :type Actor%20Object%20Reference) (OtherComp :type Primitive%20Component%20Object%20Reference) (NormalImpulse :type Vector :default "0, 0, 0") (Hit :type Hit%20Result%20Structure%20%28by%20ref%29))
  ;[1 1 1] If the peg is hit, the ball and peg are the same color and not a blocker, then call the 'Hit by Ball' function and pass in the proper color
  (bind _asbp_peggle_ball (Utilities|Casting|CastToBP_PeggleBall OtherActor))
  (if (Utilities|Enum|NotEqual(Enum) (Variables|/Game/PeggleBlueprints/BP_PeggleBall.BP_PeggleBall_C|GetBallType _asbp_peggle_ball) "NewEnumerator11")
    ;[1 1 1] If Special Ability
    (if (Utilities|Enum|Equal(Enum) (Variables|Default|GetPegType) "NewEnumerator9")
      (Utilities|FlowControl|Delay 0.2)
      (Game|SpawnActorfromClass "/Game/PeggleBlueprints/BP_ScoreText.BP_ScoreText_C" (Math|Transform|MakeTransform (Transformation|GetWorldLocation (Variables|Default|GetPeg)) "0, 0, 0" "1,1,1") "Undefined" 0 "SPECIAL!" 0)
      (Audio|PlaySound2D "/Game/Interface_and_Item_SFX_10/Items_Collectibles/cue/Special___Powerup__14__Cue.Special___Powerup__14__Cue" 1.0 1.0 0.0 0 0)
      (Game|SpawnActorfromClass "/Game/PeggleBlueprints/BP_ExplosionParticle.BP_ExplosionParticle_C" (Math|Transform|MakeTransform (Transformation|GetWorldLocation (Variables|Default|GetPeg)) "0, 0, 0" "1,1,1") "Undefined" 0 "/Game/PeggleAssets/ParticleMaterials/M_ParticleShardSpecial.M_ParticleShardSpecial" "(B=0,G=0,R=0,A=0)" 0)
      (Actor|DestroyActor)
      (elif (Utilities|Enum|NotEqual(Enum) (Variables|Default|GetPegType) "NewEnumerator0")
        (if (not (Variables|Default|GetStopHitting?))
          (bind _destroy_ (CallFunction|HitbyBall (Utilities|Select :Index (Variables|/Game/PeggleBlueprints/BP_PeggleBall.BP_PeggleBall_C|GetBallType _asbp_peggle_ball) :NewEnumerator2 "NewEnumerator2" :NewEnumerator3 "NewEnumerator3" :NewEnumerator4 "NewEnumerator4" :NewEnumerator11 "NewEnumerator0")))
          (if _destroy_
            (Utilities|FlowControl|Delay 0.2)
            (Actor|DestroyActor)))))))

(event EventBeginPlay
  ;[1 1 1] Randomize peg color unless it's already assigned as a Blocker or SpecialAbility peg.
)

(fn ConstructionScript
  ;[1 1 1] Set the peg shape and color in editor
  (Components|StaticMesh|SetStaticMesh (Variables|Default|GetPeg) (Utilities|Select :Index (Variables|Default|GetPegShape) :Option%200 "/Game/PeggleAssets/Pegs_RoundPeg.Pegs_RoundPeg" :Option%201 "/Game/PeggleAssets/Pegs_SquarePeg.Pegs_SquarePeg" :Option%202 "/Game/PeggleAssets/Pegs_RectanglePeg.Pegs_RectanglePeg"))
  (Rendering|Material|SetMaterial (Variables|Default|GetPeg) 0 (Utilities|Select :Index (Variables|Default|GetPegType) :NewEnumerator2 "/Game/PeggleAssets/PegMaterials/M_PegFlirtation.M_PegFlirtation" :NewEnumerator3 "/Game/PeggleAssets/PegMaterials/M_PegRomance.M_PegRomance" :NewEnumerator4 "/Game/PeggleAssets/PegMaterials/M_PegSexuality.M_PegSexuality" :NewEnumerator9 "/Game/PeggleAssets/PegMaterials/M_PegSpecial.M_PegSpecial" :NewEnumerator0 "/Game/PeggleAssets/PegMaterials/M_PegBlocker.M_PegBlocker")))

(fn HitbyBall
  (params (BallColor :type ETypesOfPegsEnum%20Enum :default "NewEnumerator1"))
  (bind _returnvalue (Game|GetGameInstance))
  (bind _returnvalue_2 (Game|Player|GetPlayerPawn 0))
  (bind _pegtype (Variables|Default|GetPegType))
  (bind _asbp_main_instance (Utilities|Casting|CastToBP_MainInstance _returnvalue))
  (bind _asbp_peggle_player (Utilities|Casting|CastToBP_PegglePlayer _returnvalue_2))
  (bind _currentgirl (Variables|/Game/PeggleBlueprints/PeggleData/BP_MainInstance.BP_MainInstance_C|GetCurrentGirl _asbp_main_instance))
  (bind _girl1 (Variables|/Game/PeggleBlueprints/PeggleData/BP_MainInstance.BP_MainInstance_C|GetGirl1 _asbp_main_instance))
  (bind _girl2 (Variables|/Game/PeggleBlueprints/PeggleData/BP_MainInstance.BP_MainInstance_C|GetGirl2 _asbp_main_instance))
  (bind _girl3 (Variables|/Game/PeggleBlueprints/PeggleData/BP_MainInstance.BP_MainInstance_C|GetGirl3 _asbp_main_instance))
  (bind _returnvalue_3 (Utilities|Select :Index _currentgirl :NewEnumerator0 _girl1 :NewEnumerator1 _girl2 :NewEnumerator2 _girl3))
  (bind (_likedattribute _dislikedattribute) (Utilities|Struct|BreakSGirlStruct _returnvalue_3))
  ;[1 1 1] If peg is NOT set as Type02, double check that the peg type and ball color are the same before continuing
  (if (Utilities|Enum|NotEqual(Enum) BallColor "NewEnumerator0")
    (if (Variables|Default|GetType02?)
      (Utilities|FlowControl|Sequence :!label _label
        (:then_0
          ;[1 1 1] Track number of combo hits
          (bind _output_get (Variables|/Game/PeggleBlueprints/BP_PegglePlayer.BP_PegglePlayer_C|SetComboHitNumber _asbp_peggle_player (+ (Variables|/Game/PeggleBlueprints/BP_PegglePlayer.BP_PegglePlayer_C|GetComboHitNumber _asbp_peggle_player) 1)))
          (Variables|Default|SetComboHit _output_get))
        (:then_1
          ;[1 1 1] Set default current peg value plus 1 per combo hits.
          (Variables|Default|SetPegScoreValue (+ (Variables|Default|GetDefaulPegValue) (- (Math|Conversions|ToFloat(Integer) (Variables|Default|GetComboHit)) 1.0))))
        (:then_2
          ;[1 1 1] Only do next check if peg is set as Type02
          (if (Variables|Default|GetType02?)
            ;[1 1 1] If the peg and ball are the same color, x2 peg value
            (if (Utilities|Enum|Equal(Enum) BallColor (Variables|Default|GetPegType))
              (Variables|Default|SetPegScoreValue (* (Variables|Default|GetPegScoreValue) 2.0)))))
        (:then_3
          ;[1 1 1] Overwrite the current peg value if it's either a liked or disliked color
          (if (Utilities|Enum|Equal(Enum) _likedattribute _pegtype)
            (Variables|Default|SetPegScoreValue (* (Variables|Default|GetPegScoreValue) 2.0))))
        (:then_4
          (if (Utilities|Enum|Equal(Enum) _dislikedattribute _pegtype)
            (Variables|Default|SetPegScoreValue (/ (Variables|Default|GetPegScoreValue) 2.0))))
        (:then_5
          ;[1 1 1] Calculations for points gained based on stats, passion, etc. Score added to CurrentScore in game instance. (Or CurrentPassion if it's a passion hit.)
          (switch Utilities|FlowControl|Switch|SwitchonETypesOfPegsEnum (Variables|Default|GetPegType)
            (:NewEnumerator2
              (Variables|Default|SetPegScoreValue (+ (Variables|/Game/PeggleBlueprints/PeggleData/BP_MainInstance.BP_MainInstance_C|GetFlirtationStat _asbp_main_instance) (Variables|Default|GetPegScoreValue))))
            (:NewEnumerator3
              (Variables|Default|SetPegScoreValue (+ (Variables|/Game/PeggleBlueprints/PeggleData/BP_MainInstance.BP_MainInstance_C|GetRomanceStat _asbp_main_instance) (Variables|Default|GetPegScoreValue))))
            (:NewEnumerator4
              (Variables|Default|SetPegScoreValue (+ (Variables|/Game/PeggleBlueprints/PeggleData/BP_MainInstance.BP_MainInstance_C|GetSexualityStat _asbp_main_instance) (Variables|Default|GetPegScoreValue)))))
          (bind _output_get_2 (Variables|Default|SetPegScoreValue (* (Variables|Default|GetPegScoreValue) (Variables|/Game/PeggleBlueprints/BP_PegglePlayer.BP_PegglePlayer_C|GetCurrentMultiplier (.AsBP%20Peggle%20Player (Utilities|Casting|CastToBP_PegglePlayer (Game|Player|GetPlayerPawn 0)))))))
          (Variables|/Game/PeggleBlueprints/PeggleData/BP_MainInstance.BP_MainInstance_C|SetCurrentScore _asbp_main_instance (Math|Float|Truncate (+ _output_get_2 (Math|Conversions|ToFloat(Integer) (Variables|/Game/PeggleBlueprints/PeggleData/BP_MainInstance.BP_MainInstance_C|GetCurrentScore _asbp_main_instance)))))
          ;[1 1 1] Spawn score text BP at peg location and feed it the peg score. Sent the widget a notify that a brick is broken, spawn explosion particles, destroy brick.
          (Game|SpawnActorfromClass "/Game/PeggleBlueprints/BP_ScoreText.BP_ScoreText_C" (Math|Transform|MakeTransform (Transformation|GetWorldLocation (Variables|Default|GetPeg)) "0, 0, 0" "1,1,1") "Undefined" 0 (Utilities|Text|ToText(Float) (Variables|Default|GetPegScoreValue) "HalfToEven") 0)
          (bind _foundwidgets (Widget|GetAllWidgetsOfClass "/Game/PeggleBlueprints/WBP_TestUI.WBP_TestUI_C" true))
          (for _array_element _foundwidgets
            (Class|BPIMainInterface|BrickBroken(Message) _array_element)
            (Class|BPIMainInterface|BrickBroken(Message) (.AsBP%20Peggle%20Player (Utilities|Casting|CastToBP_PegglePlayer (Game|Player|GetPlayerPawn 0))))
            (Game|SpawnActorfromClass "/Game/PeggleBlueprints/BP_ExplosionParticle.BP_ExplosionParticle_C" (Math|Transform|MakeTransform (Transformation|GetWorldLocation (Variables|Default|GetPeg)) "0, 0, 0" "1,1,1") "Undefined" 0 (Utilities|Select :Index (Variables|Default|GetPegType) :NewEnumerator2 "/Game/PeggleAssets/ParticleMaterials/M_ParticleShardFlirtation.M_ParticleShardFlirtation" :NewEnumerator3 "/Game/PeggleAssets/ParticleMaterials/M_ParticleShardRomance.M_ParticleShardRomance" :NewEnumerator4 "/Game/PeggleAssets/ParticleMaterials/M_ParticleShardSexuality.M_ParticleShardSexuality" :NewEnumerator9 "/Game/PeggleAssets/ParticleMaterials/M_ParticleShardSpecial.M_ParticleShardSpecial" :NewEnumerator0 "/Game/PeggleAssets/ParticleMaterials/M_ParticleShardDud.M_ParticleShardDud") "(B=0,G=0,R=0,A=0)" 0)
            (Audio|PlaySound2D "/Game/Interface_and_Item_SFX_10/Items_Collectibles/cue/Special___Powerup__13__Cue.Special___Powerup__13__Cue" 1.0 (+ (* (Math|Conversions|ToFloat(Integer) (Variables|Default|GetComboHit)) 0.2) 0.5) 0.0 0 0)
            (return true))))
      (elif (Utilities|Enum|Equal(Enum) BallColor _pegtype)
        (Variables|Default|SetStopHitting? true)
        (goto _label)))))

(fn SetPegMaterial
  (Rendering|Material|SetMaterial (Variables|Default|GetPeg) 0 (Utilities|Select :Index (Variables|Default|GetPegType) :NewEnumerator2 "/Game/PeggleAssets/PegMaterials/M_PegFlirtation.M_PegFlirtation" :NewEnumerator3 "/Game/PeggleAssets/PegMaterials/M_PegRomance.M_PegRomance" :NewEnumerator4 "/Game/PeggleAssets/PegMaterials/M_PegSexuality.M_PegSexuality" :NewEnumerator9 "/Game/PeggleAssets/PegMaterials/M_PegSpecial.M_PegSpecial" :NewEnumerator0 "/Game/PeggleAssets/PegMaterials/M_PegBlocker.M_PegBlocker")))