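; Peggle-style peg whose shape and type-based material are set in editor; types other than Blocker and SpecialAbility are randomized at BeginPlay.
; Ball hits score only on matching types, while SpecialAbility pegs just show text and vanish, and Blockers ignore hits.
; The current girl's likes and dislikes and player stats adjust points: Passion raises a multiplier that scales other types' score in BP_MainInstance.
; Scored pegs spawn score text, notify WBP_TestUI and destroy themselves.
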(event OnComponentHit(Peg)
  (params (HitComponent :type Primitive%20Component%20Object%20Reference) (OtherActor :type Actor%20Object%20Reference) (OtherComp :type Primitive%20Component%20Object%20Reference) (NormalImpulse :type Vector :default "0, 0, 0") (Hit :type Hit%20Result%20Structure%20%28by%20ref%29))
  ;[1 1 1] If the peg is hit, the ball and peg are the same color and not a blocker, then call the 'Hit by Ball' function and pass in the proper color
  (bind _asbp_peggle_ball (Utilities|Casting|CastToBP_PeggleBall OtherActor))
  ;[1 1 1] If Special Ability
  (if (Utilities|Enum|Equal(Enum) (Variables|Default|GetPegType) "NewEnumerator9")
    (Utilities|FlowControl|Delay 0.2)
    (Game|SpawnActorfromClass "/Game/PeggleBlueprints/BP_ScoreText.BP_ScoreText_C" (Math|Transform|MakeTransform (Transformation|GetWorldLocation (Variables|Default|GetPeg)) "0, 0, 0" "1,1,1") "Undefined" 0 "SPECIAL!" 0)
    (Actor|DestroyActor)
    (elif (Utilities|Enum|NotEqual(Enum) (Variables|Default|GetPegType) "NewEnumerator0")
      (Utilities|FlowControl|Delay 0.2)
      (CallFunction|HitbyBall (Utilities|Select :Index (Variables|/Game/PeggleBlueprints/BP_PeggleBall.BP_PeggleBall_C|GetBallType _asbp_peggle_ball) :NewEnumerator1 "NewEnumerator1" :NewEnumerator2 "NewEnumerator2" :NewEnumerator3 "NewEnumerator3" :NewEnumerator4 "NewEnumerator4" :NewEnumerator5 "NewEnumerator5")))))

(event EventBeginPlay
  ;[1 1 1] Randomize peg color unless it's already assigned as a Blocker or SpecialAbility peg.
  (if (and (Utilities|Enum|NotEqual(Enum) (Variables|Default|GetPegType) "NewEnumerator9") (Utilities|Enum|NotEqual(Enum) (Variables|Default|GetPegType) "NewEnumerator0"))
    (Variables|Default|SetPegType (Utilities|Enum|ByteToEnumETypesOfPegsEnum (Math|Conversions|ToByte(Integer) (Math|Random|RandomInteger 5))))
    (Rendering|Material|SetMaterial (Variables|Default|GetPeg) 0 (Utilities|Select :Index (Variables|Default|GetPegType) :NewEnumerator1 "/Game/PeggleAssets/PegMaterials/M_PegPassion.M_PegPassion" :NewEnumerator2 "/Game/PeggleAssets/PegMaterials/M_PegFlirtation.M_PegFlirtation" :NewEnumerator3 "/Game/PeggleAssets/PegMaterials/M_PegRomance.M_PegRomance" :NewEnumerator4 "/Game/PeggleAssets/PegMaterials/M_PegSexuality.M_PegSexuality" :NewEnumerator5 "/Game/PeggleAssets/PegMaterials/M_PegTalent.M_PegTalent" :NewEnumerator9 "/Game/PeggleAssets/PegMaterials/M_PegSpecial.M_PegSpecial" :NewEnumerator0 "/Game/PeggleAssets/PegMaterials/M_PegBlocker.M_PegBlocker" :NewEnumerator8 "/Game/PeggleAssets/PegMaterials/M_PegBrokenHeart.M_PegBrokenHeart" :NewEnumerator10 "/Game/PeggleAssets/PegMaterials/M_PegSentiment.M_PegSentiment" :NewEnumerator6 "/Game/PeggleAssets/PegMaterials/M_PegBell.M_PegBell"))))

(fn ConstructionScript
  ;[1 1 1] Set the peg shape and color in editor
  (Components|StaticMesh|SetStaticMesh (Variables|Default|GetPeg) (Utilities|Select :Index (Variables|Default|GetPegShape) :Option%200 "/Game/PeggleAssets/Pegs_RoundPeg.Pegs_RoundPeg" :Option%201 "/Game/PeggleAssets/Pegs_SquarePeg.Pegs_SquarePeg" :Option%202 "/Game/PeggleAssets/Pegs_RectanglePeg.Pegs_RectanglePeg"))
  (Rendering|Material|SetMaterial (Variables|Default|GetPeg) 0 (Utilities|Select :Index (Variables|Default|GetPegType) :NewEnumerator1 "/Game/PeggleAssets/PegMaterials/M_PegPassion.M_PegPassion" :NewEnumerator2 "/Game/PeggleAssets/PegMaterials/M_PegFlirtation.M_PegFlirtation" :NewEnumerator3 "/Game/PeggleAssets/PegMaterials/M_PegRomance.M_PegRomance" :NewEnumerator4 "/Game/PeggleAssets/PegMaterials/M_PegSexuality.M_PegSexuality" :NewEnumerator5 "/Game/PeggleAssets/PegMaterials/M_PegTalent.M_PegTalent" :NewEnumerator9 "/Game/PeggleAssets/PegMaterials/M_PegSpecial.M_PegSpecial" :NewEnumerator0 "/Game/PeggleAssets/PegMaterials/M_PegBlocker.M_PegBlocker" :NewEnumerator8 "/Game/PeggleAssets/PegMaterials/M_PegBrokenHeart.M_PegBrokenHeart" :NewEnumerator10 "/Game/PeggleAssets/PegMaterials/M_PegSentiment.M_PegSentiment" :NewEnumerator6 "/Game/PeggleAssets/PegMaterials/M_PegBell.M_PegBell")))

(fn HitbyBall
  (params (BallColor :type ETypesOfPegsEnum%20Enum :default "NewEnumerator1"))
  (bind _returnvalue (Game|GetGameInstance))
  (bind _pegtype (Variables|Default|GetPegType))
  (bind _asbp_main_instance (Utilities|Casting|CastToBP_MainInstance _returnvalue))
  (bind _currentgirl (Variables|/Game/PeggleBlueprints/PeggleData/BP_MainInstance.BP_MainInstance_C|GetCurrentGirl _asbp_main_instance))
  (bind _girl1 (Variables|/Game/PeggleBlueprints/PeggleData/BP_MainInstance.BP_MainInstance_C|GetGirl1 _asbp_main_instance))
  (bind _girl2 (Variables|/Game/PeggleBlueprints/PeggleData/BP_MainInstance.BP_MainInstance_C|GetGirl2 _asbp_main_instance))
  (bind _girl3 (Variables|/Game/PeggleBlueprints/PeggleData/BP_MainInstance.BP_MainInstance_C|GetGirl3 _asbp_main_instance))
  (bind _returnvalue_2 (Utilities|Select :Index _currentgirl :NewEnumerator0 _girl1 :NewEnumerator1 _girl2 :NewEnumerator2 _girl3))
  (bind (_likedattribute _dislikedattribute) (Utilities|Struct|BreakSGirlStruct _returnvalue_2))
  ;[1 1 1] Double check that the peg type and ball color are the same
  (if (Utilities|Enum|Equal(Enum) BallColor _pegtype)
    (Utilities|FlowControl|Sequence
      (:then_0
        ;[1 1 1] Set default current peg value
        (Variables|Default|SetPegScoreValue (Variables|Default|GetDefaulPegValue)))
      (:then_1
        ;[1 1 1] Overwrite the current peg value if it's either a liked or disliked color
        (if (Utilities|Enum|Equal(Enum) _likedattribute _pegtype)
          (Variables|Default|SetPegScoreValue (* (Variables|Default|GetDefaulPegValue) 2.0))))
      (:then_2
        (if (Utilities|Enum|Equal(Enum) _dislikedattribute _pegtype)
          (Variables|Default|SetPegScoreValue (/ (Variables|Default|GetDefaulPegValue) 2.0))))
      (:then_3
        ;[1 1 1] Calculations for points gained based on stats, passion, etc. Score added to CurrentScore in game instance. (Or CurrentPassion if it's a passion hit.)
        (switch Utilities|FlowControl|Switch|SwitchonETypesOfPegsEnum (Variables|Default|GetPegType)
          (:NewEnumerator1
            (bind _output_get (Variables|Default|SetPegScoreValue (+ (Variables|/Game/PeggleBlueprints/PeggleData/BP_MainInstance.BP_MainInstance_C|GetPassionStat _asbp_main_instance) (Variables|Default|GetPegScoreValue))))
            (bind _output_get_2 (Variables|Default|SetPegScoreValue (* _output_get 0.1)))
            (Variables|/Game/PeggleBlueprints/PeggleData/BP_MainInstance.BP_MainInstance_C|SetCurrentPassion _asbp_main_instance (+ _output_get_2 (Variables|/Game/PeggleBlueprints/PeggleData/BP_MainInstance.BP_MainInstance_C|GetCurrentPassion _asbp_main_instance))))
          (:NewEnumerator2
            (Variables|Default|SetPegScoreValue (+ (Variables|/Game/PeggleBlueprints/PeggleData/BP_MainInstance.BP_MainInstance_C|GetFlirtationStat _asbp_main_instance) (Variables|Default|GetPegScoreValue)))
            (bind _output_get_3 (Variables|Default|SetPegScoreValue (* (Variables|Default|GetPegScoreValue) (Variables|/Game/PeggleBlueprints/PeggleData/BP_MainInstance.BP_MainInstance_C|GetCurrentPassion _asbp_main_instance)) :!label _label))
            (Variables|/Game/PeggleBlueprints/PeggleData/BP_MainInstance.BP_MainInstance_C|SetCurrentScore _asbp_main_instance (Math|Float|Truncate (+ _output_get_3 (Math|Conversions|ToFloat(Integer) (Variables|/Game/PeggleBlueprints/PeggleData/BP_MainInstance.BP_MainInstance_C|GetCurrentScore _asbp_main_instance))))))
          (:NewEnumerator3
            (Variables|Default|SetPegScoreValue (+ (Variables|/Game/PeggleBlueprints/PeggleData/BP_MainInstance.BP_MainInstance_C|GetRomanceStat _asbp_main_instance) (Variables|Default|GetPegScoreValue)))
            (goto _label))
          (:NewEnumerator4
            (Variables|Default|SetPegScoreValue (+ (Variables|/Game/PeggleBlueprints/PeggleData/BP_MainInstance.BP_MainInstance_C|GetSexualityStat _asbp_main_instance) (Variables|Default|GetPegScoreValue)))
            (goto _label))
          (:NewEnumerator5
            (Variables|Default|SetPegScoreValue (+ (Variables|/Game/PeggleBlueprints/PeggleData/BP_MainInstance.BP_MainInstance_C|GetTalentStat _asbp_main_instance) (Variables|Default|GetPegScoreValue)))
            (goto _label)))
        ;[1 1 1] Spawn score text BP at peg location and feed it the peg score. Sent the widget a notify that a brick is broken, destroy brick.
        (Game|SpawnActorfromClass "/Game/PeggleBlueprints/BP_ScoreText.BP_ScoreText_C" (Math|Transform|MakeTransform (Transformation|GetWorldLocation (Variables|Default|GetPeg)) "0, 0, 0" "1,1,1") "Undefined" 0 (Utilities|Text|ToText(Float) (Variables|Default|GetPegScoreValue) "HalfToEven") 0)
        (bind _foundwidgets (Widget|GetAllWidgetsOfClass "/Game/PeggleBlueprints/WBP_TestUI.WBP_TestUI_C" true))
        (for _array_element _foundwidgets
          (Class|BPIMainInterface|BrickBroken(Message) _array_element)
          (Actor|DestroyActor))))))